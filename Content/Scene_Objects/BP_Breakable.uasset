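; BP_Breakable is a destructible block that awards points and deflects the ball when struck.
; On BeginPlay it applies its material to the cube and caches the GameManager found in the level.
; On a hit from BP_Ball, it reflects the ball's 2D direction off the impact normal with a random yaw offset.
; It then adds its Points to the manager's score and destroys itself.
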(event `self.ReceiveBeginPlay`
  (`PrimitiveComponent.SetMaterial` (`self.Cube`) 0 (`self._Material`))
  (bind _returnvalue (`GameplayStatics.GetActorOfClass` "/Game/GameManager.GameManager_C"))
  (set `self._Gm` _returnvalue))

(event `self.ReceiveHit`
  (params (MyComp :type "PrimitiveComponent Object Reference") (Other :type "Actor Object Reference") (OtherComp :type "PrimitiveComponent Object Reference") (bSelfMoved :type Boolean) (HitLocation :type "Vector Structure") (HitNormal :type "Vector Structure") (NormalImpulse :type "Vector Structure") (Hit :type "HitResult Structure (by ref)"))
  (bind _asbp_ball (cast `/Game/Scene_Objects/BP_Ball` Other))
  (bind (_returnvalue_x _returnvalue_y) (`KismetMathLibrary.BreakVector` (`KismetMathLibrary.GreaterGreater_VectorRotator` (`KismetMathLibrary.GetReflectionVector` (`KismetMathLibrary.Conv_Vector2DToVector` (`/Game/Scene_Objects/BP_Ball.2D_Dir` _asbp_ball)) (`.ImpactNormal` (`GameplayStatics.BreakHitResult` Hit))) (`KismetMathLibrary.MakeRotator` 0.0 0.0 (`KismetMathLibrary.RandomFloatInRange` -20.0 20.0)))))
  (set `/Game/Scene_Objects/BP_Ball.2D_Dir` (`KismetMathLibrary.MakeVector2D` _returnvalue_x _returnvalue_y) _asbp_ball)
  (`/Game/GameManager.AddScore` (`self._Gm`) (`self.Points`))
  (`self.K2_DestroyActor`))

(fn `UserConstructionScript`)